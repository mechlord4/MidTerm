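; Pong power-up pickup that picks a random type on BeginPlay and affects the paddle of whoever last hit.
; UsePickup checks the game mode's PlayerLastHit flag to choose the player or enemy paddle struct, then switches on the type to set speed or size.
; Speed and size types then call SpeedUpPickup or SizePickUp on that paddle actor.
; Ice only sets the player's Icy flag and has no enemy branch.
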(event `self.ReceiveBeginPlay`
  (set `self.PickupType` (cast `/Game/PowerUpList` (`KismetMathLibrary.Conv_IntToByte` (`KismetMathLibrary.RandomIntegerInRange` 0 (- (enumcount `/Game/PowerUpList`) 1))))))

(event `UsePickup`
  (bind _pickuptype (`self.PickupType`))
  (bind _aspong_game_mode (cast `/Game/PongGameMode` (`GameplayStatics.GetGameMode`)))
  (if (`/Game/PongGameMode.PlayerLastHit` _aspong_game_mode)
    (switch `/Game/PowerUpList` _pickuptype
      (:`NewEnumerator0`
        (bind _playerpaddleinfor (`/Game/PongGameMode.PlayerPaddleInfor` _aspong_game_mode))
        (setmembers `/Game/PaddleStruct` :`StructRef` _playerpaddleinfor :`SPEED` 1.5)
        (bind _paddleactor (break `/Game/PaddleStruct` _playerpaddleinfor))
        (`/Game/Player.SpeedUpPickup` _paddleactor :!label _label))
      (:`NewEnumerator1`
        (setmembers `/Game/PaddleStruct` :`StructRef` _playerpaddleinfor :`SPEED` 0.5)
        (goto _label))
      (:`NewEnumerator2`
        (setmembers `/Game/PaddleStruct` :`StructRef` _playerpaddleinfor :`Size` 2.0)
        (`/Game/Player.SizePickUp` _paddleactor :!label _label_2))
      (:`NewEnumerator3`
        (setmembers `/Game/PaddleStruct` :`StructRef` _playerpaddleinfor :`Size` 0.5)
        (goto _label_2))
      (:`NewEnumerator4`
        (setmembers `/Game/PaddleStruct` :`StructRef` _playerpaddleinfor :`Icy` true)))
    (else
      (switch `/Game/PowerUpList` _pickuptype
        (:`NewEnumerator0`
          (bind _enemypaddleinfo (`/Game/PongGameMode.EnemyPaddleInfo` _aspong_game_mode))
          (setmembers `/Game/EnemyStruct` :`StructRef` _enemypaddleinfo :`Speed` 1.5)
          (bind _paddleactor_2 (break `/Game/EnemyStruct` _enemypaddleinfo))
          (`/Game/Ai.SpeedUpPickup` _paddleactor_2 :!label _label_3))
        (:`NewEnumerator1`
          (setmembers `/Game/EnemyStruct` :`StructRef` _enemypaddleinfo :`Speed` 0.5)
          (goto _label_3))
        (:`NewEnumerator2`
          (setmembers `/Game/EnemyStruct` :`StructRef` _enemypaddleinfo :`Size` 2.0)
          (`/Game/Ai.SizePickUp` _paddleactor_2 :!label _label_4))
        (:`NewEnumerator3`
          (setmembers `/Game/EnemyStruct` :`StructRef` _enemypaddleinfo :`Size` 0.5)
          (goto _label_4))))))

(fn `UserConstructionScript`)
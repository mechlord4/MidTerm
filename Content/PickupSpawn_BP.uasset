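; Spawner actor that periodically drops PickUp_BP pickups at random points inside a box volume for as long as it runs.
; The construction script sizes the Box component from the BoxExtent variable, which also bounds the random spawn point around the actor's location.
; After an initial random delay on BeginPlay, the SpawnTine event spawns a pickup, waits another random delay and calls itself again in an endless loop.
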(event `self.ReceiveBeginPlay`
  (`KismetSystemLibrary.Delay` (`KismetMathLibrary.RandomFloatInRange` 10.0 20.0))
  (`self.SpawnTine`))

(event `SpawnTine`
  (`|SpawnActorFromClass` "/Game/PickUp_BP.PickUp_BP_C" (`KismetMathLibrary.MakeTransform` (`KismetMathLibrary.RandomPointInBoundingBox` (`self.K2_GetActorLocation`) (`self.BoxExtent`))) "Undefined" "MultiplyWithRoot" null null)
  (`KismetSystemLibrary.Delay` (`KismetMathLibrary.RandomFloatInRange` 10.0 20.0))
  (`self.SpawnTine`))

(fn `UserConstructionScript`
  (`BoxComponent.SetBoxExtent` (`self.Box`) (`self.BoxExtent`) true))